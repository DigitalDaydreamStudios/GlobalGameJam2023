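; GoalShip is the level goal actor that completes the level when the player pawn overlaps its GoalPlane.
; CompleteLevel finds the current level's name among the ordered rows of DT_LevelsList and opens the level in the following row.
; On the last row it calls WinGame, which shows the WID_WinScreen widget.
; Debug prints report overlaps and level transitions.
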(event OnComponentBeginOverlap(GoalPlane)
  (params (OverlappedComponent :type Primitive%20Component%20Object%20Reference) (OtherActor :type Actor%20Object%20Reference) (OtherComp :type Primitive%20Component%20Object%20Reference) (OtherBodyIndex :type Integer) (bFromSweep :type Boolean) (SweepResult :type Hit%20Result%20Structure%20%28by%20ref%29))
  (if (and (== OverlappedComponent (Variables|Default|GetGoalPlane)) (== OtherActor (Game|Player|GetPlayerPawn 0)))
    (CallFunction|CompleteLevel)))

(event EventBeginPlay)

(event EventTick
  (params (DeltaSeconds :type Float%20%28single-precision%29)))

(event Collision|EventActorBeginOverlap
  (params (OtherActor :type Actor%20Object%20Reference))
  (Development|PrintString "Overlapping with Player" (Collision|IsOverlappingActor OtherActor (Game|Player|GetPlayerPawn 0) :!class /Script/Engine.Actor)))

(fn ConstructionScript)

(fn CompleteLevel
  (bind _returnvalue (Game|GetCurrentLevelName true))
  (bind _outrownames (DataTable|GetDataTableRowNames "/Game/Data/DT_LevelsList.DT_LevelsList"))
  (bind (_array_element _array_index) (Utilities|Array|ForEachLoopwithBreak _outrownames :!label _label)
    (:LoopBody
      (bind _returnvalue_2 (Utilities|GetDataTableRow "/Game/Data/DT_LevelsList.DT_LevelsList" _array_element)
        (:then
          (Development|PrintString (Utilities|String|ToString(Name) (.levelname _returnvalue_2)))
          (if (Utilities|Enum|Equal(Enum) _returnvalue (Utilities|String|ToString(Name) (.levelname _returnvalue_2)))
            (if (!= (+ _array_index 1) (Utilities|Array|Length _outrownames)) ; If the next one isn't outside of bounds
              (Development|PrintString "Going to a new level")
              (bind _returnvalue_3 (Utilities|GetDataTableRow "/Game/Data/DT_LevelsList.DT_LevelsList" (Utilities|Array|Get(acopy) _outrownames (+ _array_index 1)))
                (:then
                  (Game|OpenLevel(byName) (.levelname _returnvalue_3))
                  (goto _label Break)))
              (else
                (CallFunction|WinGame)))))))))

(fn WinGame
  (Development|PrintString "You Win the game")
  (bind _returnvalue (UserInterface|CreateWidget "/Game/UI/Widgets/WID_WinScreen.WID_WinScreen_C"))
  (UserInterface|Viewport|AddtoViewport _returnvalue 0))