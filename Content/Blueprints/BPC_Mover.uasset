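; Actor component that moves and rotates its owner between its starting transform and an offset location and target rotation.
; Tick advances separate move and rotate timers, looping or ping-ponging, then lerps world transform by their clamped ratios.
; MoveOnPlayer limits motion to while PlayerInteracting is set, cleared after a delay, with optional rewind to start.
; The overlap handlers that set that flag have unconnected bindings, so another source must set it.
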(event Custom|Reset
  (Variables|Default|SetTimePassedMove 0.0)
  (Variables|Default|SetTimePassedRotate 0.0))

(event Custom|OnActorBeginOverlap_Event_0
  (params (OverlappedActor :type Actor%20Object%20Reference) (OtherActor :type Actor%20Object%20Reference))
  (Utilities|Casting|CastToCharacter OtherActor)
  (Variables|Default|SetPlayerInteracting true))

(event Custom|OnActorEndOverlap_Event_0
  (params (OverlappedActor :type Actor%20Object%20Reference) (OtherActor :type Actor%20Object%20Reference))
  (Utilities|Casting|CastToCharacter OtherActor)
  (Variables|Default|SetPlayerInteracting false))

(event EventBeginPlay
  (bind _output_get (Variables|Default|SetOwnerActor (Components|GetOwner)))
  (Variables|Default|SetStartingPoint (Transformation|GetActorLocation _output_get))
  (Variables|Default|SetStartingRotation (Transformation|GetActorRotation _output_get))
  (bind _asstatic_mesh_actor (Utilities|Casting|CastToStaticMeshActor (Variables|Default|GetOwnerActor)))
  (Transformation|SetMobility _asstatic_mesh_actor "Movable"))

(event EventTick
  (params (DeltaSeconds :type Float%20%28single-precision%29))
  (Variables|Default|SetDeltaTime DeltaSeconds)
  (if (Variables|Default|GetMoveOnPlayer)
    (if (Variables|Default|GetPlayerInteracting)
      (if (Variables|Default|GetPingPongMove) :!label _label
        (CallFunction|PingPongMoveFunction)
        (else
          (CallFunction|LinearTimeMove)))
      (if (Variables|Default|GetPingPongRotate)
        (CallFunction|PingPongRotateFunction)
        (else
          (CallFunction|LinearTimeRotate)))
      (CallFunction|UpdateRotation :!label _label_2)
      (CallFunction|UpdateLocation)
      (Utilities|FlowControl|Delay (Variables|Default|GetPlayerInteractingDelay))
      (Variables|Default|SetPlayerInteracting false)
      (elif (Variables|Default|GetReturnToStart)
        (CallFunction|TimePassedto0)
        (goto _label_2)))
    (else
      (goto _label))))

(fn PingPongMoveFunction
  (bind _deltatime (Variables|Default|GetDeltaTime))
  (if (Variables|Default|GetDirectionMove)
    (if (>= (Variables|Default|GetTotalTimeMove) (Variables|Default|GetTimePassedMove))
      (Variables|Default|SetTimePassedMove (+ _deltatime (Variables|Default|GetTimePassedMove)))
      (else
        (Variables|Default|SetDirectionMove false)))
    (elif (>= (Variables|Default|GetTimePassedMove) 0.0)
      (Variables|Default|SetTimePassedMove (- (Variables|Default|GetTimePassedMove) _deltatime))
      (else
        (Variables|Default|SetDirectionMove true)))))

(fn PingPongRotateFunction
  (bind _deltatime (Variables|Default|GetDeltaTime))
  (if (Variables|Default|GetDirectionRotate)
    (if (>= (Variables|Default|GetTotalTimeRotate) (Variables|Default|GetTimePassedRotate))
      (Variables|Default|SetTimePassedRotate (+ _deltatime (Variables|Default|GetTimePassedRotate)))
      (else
        (Variables|Default|SetDirectionRotate false)))
    (elif (>= (Variables|Default|GetTimePassedRotate) 0.0)
      (Variables|Default|SetTimePassedRotate (- (Variables|Default|GetTimePassedRotate) _deltatime))
      (else
        (Variables|Default|SetDirectionRotate true)))))

(fn LinearTimeMove
  (if (>= (Variables|Default|GetTotalTimeMove) (Variables|Default|GetTimePassedMove))
    (Variables|Default|SetTimePassedMove (+ (Variables|Default|GetdeltaTime) (Variables|Default|GetTimePassedMove)))
    (else
      (Variables|Default|SetTimePassedMove 0.0))))

(fn LinearTimeRotate
  (if (>= (Variables|Default|GetTotalTimeRotate) (Variables|Default|GetTimePassedRotate))
    (Variables|Default|SetTimePassedRotate (+ (Variables|Default|GetdeltaTime) (Variables|Default|GetTimePassedRotate)))
    (else
      (Variables|Default|SetTimePassedRotate 0.0))))

(fn TimePassedto0
  (if (>= (Variables|Default|GetTimePassedMove) 0.0)
    (Variables|Default|SetTimePassedMove (- (Variables|Default|GetTimePassedMove) (Variables|Default|GetdeltaTime))))
  (if (>= (Variables|Default|GetTimePassedRotate) 0.0)
    (Variables|Default|SetTimePassedRotate (- (Variables|Default|GetTimePassedRotate) (Variables|Default|GetdeltaTime)))))

(fn UpdateLocation
  (Transformation|SetWorldLocation (Variables|/Script/Engine.Actor|GetRootComponent (Variables|Default|GetOwnerActor)) (Math|Vector|Lerp(Vector) (Variables|Default|GetStartingPoint) (+ (Variables|Default|GetStartingPoint) (Variables|Default|GetEndingPoint)) (Math|Float|Clamp(Float) (/ (Variables|Default|GetTimePassedMove) (Variables|Default|GetTotalTimeMove)) 0.0 0.9999)) false false))

(fn UpdateRotation
  (Transformation|SetWorldRotation (Variables|/Script/Engine.Actor|GetRootComponent (Variables|Default|GetOwnerActor)) (Math|Rotator|Lerp(Rotator) (Variables|Default|GetStartingRotation) (Variables|Default|GetEndRotation) (Math|Float|Clamp(Float) (/ (Variables|Default|GetTimePassedRotate) (Variables|Default|GetTotalTimeRotate)) 0.0 0.9999)) false false))