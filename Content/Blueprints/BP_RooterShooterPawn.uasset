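; Player pawn Blueprint for RooterShooter that handles the player's death and level restart.
; BlewUp disables input, hides the mesh, plays an explosion sound and emitter, then fades the camera out before reloading the current level.
; FadedAway runs the same input lock, fade and delayed reload without the explosion, while Reset reloads the level immediately.
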(event Custom|BlewUp
  (bind _camerafadeduration (Variables|Default|GetCameraFadeDuration))
  (Input|DisableInput (Game|GetPlayerController 0))
  (Rendering|SetVisibility (Variables|Default|GetStaticMesh) false false)
  (Audio|SpawnSound2D "/Game/Audio/explosion_deep_low_1.explosion_deep_low_1" 1.0 1.0 0.0 0)
  (Effects|SpawnEmitteratLocation "/Game/FXVarietyPack/Particles/P_ky_explosion.P_ky_explosion" (Transformation|GetActorLocation))
  (CameraFades|StartCameraFade :self (Game|GetPlayerCameraManager 0) :ToAlpha 1.0 :Duration _camerafadeduration :bHoldWhenFinished true)
  (Utilities|FlowControl|Delay (+ _camerafadeduration (Variables|Default|GetDeathDelay)))
  (bind _returnvalue (Game|GetCurrentLevelName true))
  (Game|OpenLevel(byName) (Utilities|String|StringToName _returnvalue)))

(event Custom|FadedAway
  (bind _camerafadeduration (Variables|Default|GetCameraFadeDuration))
  (Input|DisableInput (Game|GetPlayerController 0))
  (CameraFades|StartCameraFade :self (Game|GetPlayerCameraManager 0) :ToAlpha 1.0 :Duration _camerafadeduration :bHoldWhenFinished true)
  (Utilities|FlowControl|Delay (+ _camerafadeduration (Variables|Default|GetDeathDelay)))
  (bind _returnvalue (Game|GetCurrentLevelName true))
  (Game|OpenLevel(byName) (Utilities|String|StringToName _returnvalue)))

(event EventBeginPlay)

(event Collision|EventActorBeginOverlap
  (params (OtherActor :type Actor%20Object%20Reference)))

(event EventTick
  (params (DeltaSeconds :type Float%20%28single-precision%29)))

(event EventReset
  (bind _returnvalue (Game|GetCurrentLevelName true))
  (Game|OpenLevel(byName) (Utilities|String|StringToName _returnvalue)))

(fn ConstructionScript)