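; BP_SpeedRing is a boost ring that pushes the player's BP_RooterShooterPawn when the pawn overlaps it.
; The Ring component's begin-overlap event ignores actors other than player pawn 0, then adds an impulse to that pawn's capsule along the ring's forward vector, scaled by the Velocity variable.
; The impulse is mass-dependent rather than a velocity change, and a 2D sci-fi sound plays with each boost.
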(event OnComponentBeginOverlap(Ring)
  (params (OverlappedComponent :type Primitive%20Component%20Object%20Reference) (OtherActor :type Actor%20Object%20Reference) (OtherComp :type Primitive%20Component%20Object%20Reference) (OtherBodyIndex :type Integer) (bFromSweep :type Boolean) (SweepResult :type Hit%20Result%20Structure%20%28by%20ref%29))
  (bind _returnvalue (Game|Player|GetPlayerPawn 0))
  (if (== OtherActor _returnvalue)
    (bind _asbp_rooter_shooter_pawn (Utilities|Casting|CastToBP_RooterShooterPawn _returnvalue))
    (Physics|AddImpulse (Variables|/Script/GlobalGameJam2023.RooterShooterPawn|GetCapsule _asbp_rooter_shooter_pawn) (* (Variables|Default|GetVelocity) (Math|Vector|GetForwardVector (Transformation|GetWorldRotation (Variables|Default|GetRing)))) "None" false)
    (Audio|PlaySound2D "/Game/Audio/sci-fi_shield_device_small_03.sci-fi_shield_device_small_03" 0.5 1.0 0.0 0 0)))

(event EventBeginPlay)

(event Collision|EventActorBeginOverlap
  (params (OtherActor :type Actor%20Object%20Reference)))

(event EventTick
  (params (DeltaSeconds :type Float%20%28single-precision%29)))

(fn ConstructionScript)